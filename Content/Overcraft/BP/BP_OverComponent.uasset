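; BP_OverComponent is a hover thruster component that tells its owning actor how hard to push upward based on ground proximity.
; Each tick it line-traces straight down along world Z for a set distance, with a one-frame debug draw.
; On a hit, a float curve maps normalized hit time to a fraction of Power, sent with itself to the owner via ReciveOverPushMessage.
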(event EventTick
  (params (DeltaSeconds :type Float%20%28single-precision%29))
  (bind (_start _end) (CallFunction|Start/endArrays))
  (bind (_outhit _returnvalue) (Collision|LineTraceByChannel _start _end "TraceTypeQuery1" true 0 "ForOneFrame"))
  (if _returnvalue
    (Class|BPIOverInterface|ReciveOverPush(Message) (Components|GetOwner) (Math|Vector|MakeVector 0.0 0.0 (Math|Float|Lerp 0.0 (Variables|Default|GetPower) (Math|Curves|GetFloatValue (Variables|Default|GetCurve) (.time _outhit)))) self)))

(fn Start/endArrays
  (return (Transformation|GetWorldLocation) (- (Transformation|GetWorldLocation) (Math|Vector|MakeVector 0.0 0.0 (Variables|Default|GetDIstance)))))